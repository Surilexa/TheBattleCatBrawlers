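; BP_Player is the player character, a side-to-side runner and jumper animated with Paper2D flipbooks.
; BeginPlay adds the Enhanced Input mapping context after a brief delay.
; Move input drives movement along the actor's forward vector, and jump input starts and stops jumping.
; Both set a movement state that swaps idle, run or jump flipbooks, with both run directions sharing one flipbook and no flip logic.
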(event Input|EnhancedActionEvents|EnhancedInputActionIA_Move
  (params (ActionValue :type Float%20%28double-precision%29) (ElapsedSeconds :type Float%20%28double-precision%29) (TriggeredSeconds :type Float%20%28double-precision%29) (InputAction :type Input%20Action%20Object%20Reference :default "/Game/Blueprints/Inputs/IA_Move.IA_Move"))
  (:Triggered
    (Pawn|Input|AddMovementInput (Transformation|GetActorForwardVector) ActionValue false)
    (if (> ActionValue 0.0)
      (CallFunction|FSetMovementState "NewEnumerator1")
      (elif (< ActionValue 0.0)
        (CallFunction|FSetMovementState "NewEnumerator2"))))
  (:Completed
    (CallFunction|FSetMovementState "NewEnumerator0")))

(event Input|EnhancedActionEvents|EnhancedInputActionIA_Jump
  (params (ActionValue :type Float%20%28double-precision%29) (ElapsedSeconds :type Float%20%28double-precision%29) (TriggeredSeconds :type Float%20%28double-precision%29) (InputAction :type Input%20Action%20Object%20Reference :default "/Game/Blueprints/Inputs/IA_Jump.IA_Jump"))
  (:Triggered
    (Character|Jump)
    (CallFunction|FSetMovementState "NewEnumerator3"))
  (:Completed
    (Character|StopJumping)
    (CallFunction|FSetMovementState "NewEnumerator0")))

(event EventBeginPlay
  (Utilities|FlowControl|Delay 0.01)
  (bind _aspc_player (Utilities|Casting|CastToPC_Player (Game|GetPlayerController 0)))
  (Utilities|IsValid _aspc_player
    (:Is%20Valid
      (Utilities|IsValid (PlayerController|LocalPlayerSubsystems|GetEnhancedInputLocalPlayerSubsystem _aspc_player)
        (:Is%20Valid
          (Input|AddMappingContext (PlayerController|LocalPlayerSubsystems|GetEnhancedInputLocalPlayerSubsystem _aspc_player) "/Game/Blueprints/IMC_Player.IMC_Player" 0 "(bIgnoreAllPressedKeysUntilRelease=True,bForceImmediately=False,bNotifyUserSettings=False)"))))))

(fn ConstructionScript)

(fn FSetMovementState
  (params (MovementAnims :type E_Animations%20Enum :default "NewEnumerator0"))
  (bind _sprite (Variables|Default|GetSprite))
  (switch Utilities|FlowControl|Switch|SwitchonE_Animations MovementAnims
    (:NewEnumerator0
      (Sprite|SetFlipbook _sprite "/Game/Flipbooks/fb_Idle.fb_Idle"))
    (:NewEnumerator1
      (Sprite|SetFlipbook _sprite "/Game/Flipbooks/fb_Run.fb_Run"))
    (:NewEnumerator2
      (Sprite|SetFlipbook _sprite "/Game/Flipbooks/fb_Run.fb_Run"))
    (:NewEnumerator3
      (Sprite|SetFlipbook _sprite "/Game/Flipbooks/fb_Jump.fb_Jump"))))